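; Player component on BP_ThirdPersonCharacter that previews and spawns a placeable platform, keeping one at a time.
; Holding IA_PlacePlatform removes the previous platform and enables placing mode; releasing spawns BP_PlacingPlatform at the last preview transform.
; Tick updates the preview only for the Green player color with the color menu closed.
; A resettable DoOnce creates the collision-free preview mesh, positioned ahead of the first-person camera at a height below the actor.
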(event `self.ReceiveBeginPlay`
  (bind _asbp_third_person_character (cast `/Game/ThirdPerson/Blueprints/BP_ThirdPersonCharacter` (`self.GetOwner`)))
  (bind _output_get (set `self.PlayerRef` _asbp_third_person_character))
  (set `self.First Person Camera` (`/Game/ThirdPerson/Blueprints/BP_ThirdPersonCharacter.FirstPersonCamera` _output_get)))

(event `Preview Loop`
  (bind _first_person_camera (`self.First Person Camera`))
  (bind (_returnvalue_x _returnvalue_y _returnvalue_z) (`KismetMathLibrary.BreakVector` (`Actor.K2_GetActorLocation` (`self.PlayerRef`))))
  (bind (_returnvalue_x_2 _returnvalue_y_2) (`KismetMathLibrary.BreakVector` (+ (`SceneComponent.K2_GetComponentLocation` _first_person_camera) (* (`SceneComponent.GetForwardVector` _first_person_camera) (`self.PlacingDistance`)))))
  (`|ExecutionSequence`
    (:`then_0`
      (`/Engine/EditorBlueprintResources/StandardMacros.DoOnce` false :!label _label
        (:`Completed`
          (bind _returnvalue (`|AddComponentByClass` (`self.PlayerRef`) "/Script/Engine.StaticMeshComponent" false (`self.PlacingPreviewTransform`)))
          (bind _output_get (set `self.PreviewMesh` _returnvalue))
          (`StaticMeshComponent.SetStaticMesh` _output_get "/Game/StarterContent/Architecture/SM_AssetPlatform.SM_AssetPlatform")
          (`PrimitiveComponent.SetMaterial` (`self.PreviewMesh`) 0 "/Engine/EditorResources/FieldNodes/_Resources/M_FieldRadiusPreview.M_FieldRadiusPreview")
          (`PrimitiveComponent.SetCollisionEnabled` (`self.PreviewMesh`) "NoCollision"))))
    (:`then_1`
      (bind _output_get_2 (set `self.PlacingPreviewTransform` (`KismetMathLibrary.MakeTransform` (`KismetMathLibrary.MakeVector` _returnvalue_x_2 _returnvalue_y_2 (+ -90.0 _returnvalue_z)))))
      (`SceneComponent.K2_SetWorldTransform` (`self.PreviewMesh`) _output_get_2 false false))))

(event `ResetPlacingMode`
  (goto _label :!via `Reset`))

(event `self.ReceiveTick`
  (params (DeltaSeconds :type "Float (single-precision)"))
  (bind _playerref (`self.PlayerRef`)
    (:`then`
      (if (and (not (`/Game/ThirdPerson/Blueprints/BP_ThirdPersonCharacter.isChangeColorMenuOpen` _playerref)) (`self.isInPlacingMode`))
        (switch `/Game/ThirdPerson/E_PlayerColor` (`/Game/Blueprints/MyGameInstance.PlayerColor` (cast `/Game/Blueprints/MyGameInstance` (`GameplayStatics.GetGameInstance`) :!pure true))
          (:`NewEnumerator2`
            (`self.Preview Loop`)))))
    (:`else`)))

(event `StopPlacingMode`
  (set `self.isInPlacingMode` false)
  (bind _previewmesh (`self.PreviewMesh`)
    (:`then`
      (`StaticMeshComponent.SetStaticMesh` _previewmesh null)
      (set `self.PreviewMesh` null)
      (`self.ResetPlacingMode`))
    (:`else`)))

(event `EnhancedInput|/Game/ThirdPerson/Input/Actions/IA_PlacePlatform`
  (params (ActionValue :type Boolean) (ElapsedSeconds :type "Float (double-precision)") (TriggeredSeconds :type "Float (double-precision)") (InputAction :type "InputAction Object Reference" :default "/Game/ThirdPerson/Input/Actions/IA_PlacePlatform.IA_PlacePlatform"))
  ; HandlingControls
  (:`Started`
    (if (`KismetSystemLibrary.IsValid` (`self.SpawnedPlatform`))
      (`Actor.K2_DestroyActor` (`self.SpawnedPlatform`)))
    (set `self.isInPlacingMode` true)
    (if (`KismetSystemLibrary.IsValid` (`self.PreviewMesh`))
      (`self.K2_DestroyComponent` (`self.PreviewMesh`))
      (else
        (bind _previewmesh (`self.PreviewMesh`)
          (:`then`
            (`StaticMeshComponent.SetStaticMesh` _previewmesh null)
            (set `self.PreviewMesh` null)
            (`self.ResetPlacingMode`))
          (:`else`))))))

(event `EnhancedInput|/Game/ThirdPerson/Input/Actions/IA_PlacePlatform`
  (params (ActionValue :type Boolean) (ElapsedSeconds :type "Float (double-precision)") (TriggeredSeconds :type "Float (double-precision)") (InputAction :type "InputAction Object Reference" :default "/Game/ThirdPerson/Input/Actions/IA_PlacePlatform.IA_PlacePlatform"))
  ; HandlingControls
  (:`Completed`
    (if (`KismetSystemLibrary.IsValid` (`self.SpawnedPlatform`))
      (`Actor.K2_DestroyActor` (`self.SpawnedPlatform`))
      (else
        (bind _returnvalue (`|SpawnActorFromClass` "/Game/PlacingPlatform/BP_PlacingPlatform.BP_PlacingPlatform_C" (`self.PlacingPreviewTransform`) "AlwaysSpawn" "MultiplyWithRoot" null null))
        (set `self.SpawnedPlatform` _returnvalue)
        (bind _previewmesh (`self.PreviewMesh`)
          (:`then`
            (`self.K2_DestroyComponent` _previewmesh)
            (`self.StopPlacingMode`)
            (set `self.isInPlacingMode` false))
          (:`else`))))))