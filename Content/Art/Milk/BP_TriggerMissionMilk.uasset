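; A milk mission trigger that acts as a pickup and completes the level when the player character touches it.
; On collision box overlap it increments the ThirdPersonCharacter's Pickups counter and destroys itself.
; With at least one pickup, it shows the WB_WinCondition widget and opens the referenced level right away, with no delay.
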(event `self.CollisionBox.OnComponentBeginOverlap`
  (params (OverlappedComponent :type "PrimitiveComponent Object Reference") (OtherActor :type "Actor Object Reference") (OtherComp :type "PrimitiveComponent Object Reference") (OtherBodyIndex :type Integer) (bFromSweep :type Boolean) (SweepResult :type "HitResult Structure (by ref)"))
  (bind _asbp_third_person_character (cast `/Game/ThirdPerson/Blueprints/BP_ThirdPersonCharacter` OtherActor))
  (bind _pickups (`/Game/ThirdPerson/Blueprints/BP_ThirdPersonCharacter.Pickups` _asbp_third_person_character))
  (set `/Game/ThirdPerson/Blueprints/BP_ThirdPersonCharacter.Pickups` (+ _pickups 1) _asbp_third_person_character)
  (`self.K2_DestroyActor`)
  (if (>= _pickups 1)
    (bind _returnvalue (`|CreateWidget` "/Game/UI/WB_WinCondition.WB_WinCondition_C"))
    (`UserWidget.AddToViewport` _returnvalue 0)
    (`/Engine/EditorBlueprintResources/StandardMacros.IsValid` OtherActor
      (:`Is Valid`
        (`GameplayStatics.OpenLevelBySoftObjectPtr` (`self.Level`))))))

(fn `UserConstructionScript`)