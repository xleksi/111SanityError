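; AI controller for the flower NPC that runs its behavior tree and tracks whether it senses the player.
; It starts BT_AI_Flower on BeginPlay.
; AI perception updates for actors tagged "player" set the "flowerseesplayer" blackboard bool to match whether sensing succeeded.
; An AiSpeed function is only a stub that ignores its input and returns zero.
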(event `self.ReceiveBeginPlay`
  (`self.RunBehaviorTree` "/Game/Art/NPC/Flower/anim3D/BT_AI_Flower.BT_AI_Flower"))

(event `self.AIPerception.OnTargetPerceptionUpdated`
  (params (Actor :type "Actor Object Reference") (Stimulus :type "AIStimulus Structure"))
  (if (`self.ActorHasTag` Actor "player")
    (if (`.bSuccessfullySensed` (break `AIStimulus` Stimulus))
      (`BlackboardComponent.SetValueAsBool` (`AIBlueprintHelperLibrary.GetBlackboard` null) "flowerseesplayer" true)
      (else
        (`BlackboardComponent.SetValueAsBool` (`AIBlueprintHelperLibrary.GetBlackboard` null) "flowerseesplayer" false)))))

(fn `ai speed`
  (params (speed :type "Float (double-precision)"))
  (returns (`amount of speed` :type "Float (double-precision)"))
  (return 0.0))

(fn `UserConstructionScript`)