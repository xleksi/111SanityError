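; BP_AI_Sun is an enemy NPC character that drains the player's sanity nearby and can kill them.
; Its InsanityArea overlap toggles GettingInsane on the player and calls FlowermanDamage on entry, while PawnSensing plays white noise on sighting through a DoOnce with retriggerable-delay reset.
; The Killa event disables input, blends the camera to itself, plays a magic attack montage and reloads the level.
; AiSpeed sets its walk speed.
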(event `self.killa`
  ;[0.15 0.01901 0.01901 0.5] AttackWhenHeCatchsU
  (`self.DisableInput` (`GameplayStatics.GetPlayerController` 0))
  (`PlayerController.SetViewTargetWithBlend` (`GameplayStatics.GetPlayerController` 0) self 10.0 "VTBlend_Linear" 0.0 false)
  (`KismetSystemLibrary.Delay` 0.3)
  (`|PlayMontage` (`self.Mesh`) "/Game/Art/NPC/Flower/anim3D/AM_magic_attack.AM_magic_attack"
    (:`then`
      (`KismetSystemLibrary.Delay` 1.6)
      (bind _returnvalue (`GameplayStatics.GetCurrentLevelName` true))
      (`GameplayStatics.OpenLevel` (`KismetStringLibrary.Conv_StringToName` _returnvalue)))))

(event `self.InsanityArea.OnComponentBeginOverlap`
  (params (OverlappedComponent :type "PrimitiveComponent Object Reference") (OtherActor :type "Actor Object Reference") (OtherComp :type "PrimitiveComponent Object Reference") (OtherBodyIndex :type Integer) (bFromSweep :type Boolean) (SweepResult :type "HitResult Structure (by ref)"))
  (bind _asbp_third_person_character (cast `/Game/ThirdPerson/Blueprints/BP_ThirdPersonCharacter` OtherActor))
  (set `/Game/ThirdPerson/Blueprints/BP_ThirdPersonCharacter.GettingInsane?` true _asbp_third_person_character)
  (`/Game/ThirdPerson/Blueprints/BP_ThirdPersonCharacter.FlowermanDamage` _asbp_third_person_character))

(event `self.InsanityArea.OnComponentEndOverlap`
  (params (OverlappedComponent :type "PrimitiveComponent Object Reference") (OtherActor :type "Actor Object Reference") (OtherComp :type "PrimitiveComponent Object Reference") (OtherBodyIndex :type Integer))
  (bind _asbp_third_person_character (cast `/Game/ThirdPerson/Blueprints/BP_ThirdPersonCharacter` OtherActor))
  (set `/Game/ThirdPerson/Blueprints/BP_ThirdPersonCharacter.GettingInsane?` false _asbp_third_person_character))

(event `self.PawnSensing.OnSeePawn`
  (params (Pawn :type "Pawn Object Reference"))
  (cast `/Game/ThirdPerson/Blueprints/BP_ThirdPersonCharacter` Pawn)
  (`|ExecutionSequence`
    (:`then_0`
      (`|ExecutionSequence`
        (:`then_0`
          (`/Engine/EditorBlueprintResources/StandardMacros.DoOnce` false :!label _label
            (:`Completed`
              (`GameplayStatics.PlaySoundAtLocation` "/Engine/EngineSounds/WhiteNoise.WhiteNoise" (`self.K2_GetActorLocation`) (struct) 1.0 1.0 3.0 null null null null))))
        (:`then_1`
          (`KismetSystemLibrary.RetriggerableDelay` 0.0)
          (goto _label :!via `Reset`))))))

(fn `ai speed`
  (params (speed :type "Float (double-precision)"))
  (returns (`amount of speed` :type "Float (double-precision)"))
  (bind _output_get (set `CharacterMovementComponent.MaxWalkSpeed` speed (`self.CharacterMovement`)))
  (return _output_get))

(fn `UserConstructionScript`)