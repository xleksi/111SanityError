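; BP_Flower2D_3 is a 2D flower hazard that turns to face the player every tick and attaches a particle effect to its sphere.
; Entering the sphere sets the player character's InsanerByFlower2D flag and calls InsanityRange.
; Leaving sets the same flag to true again rather than clearing it.
; Looping damage, sanity regeneration and flower animation logic exist but are disconnected.
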(event `self.ReceiveTick`
  (params (DeltaSeconds :type "Float (single-precision)"))
  (bind _returnvalue (`GameplayStatics.GetPlayerCharacter` 0))
  ; rotate
  (if (`KismetSystemLibrary.IsValid` _returnvalue)
    (`self.K2_SetActorRotation` (`KismetMathLibrary.FindLookAtRotation` (`self.K2_GetActorLocation`) (`self.K2_GetActorLocation` _returnvalue)))))

(event `self.ReceiveBeginPlay`
  (`GameplayStatics.SpawnEmitterAttached` null (`self.Sphere`)))

(event `Damage`
  (`GameplayStatics.ApplyDamage` (`self.ref Third Person Character`) 40.0))

(event `self.Sphere.OnComponentBeginOverlap`
  (params (OverlappedComponent :type "PrimitiveComponent Object Reference") (OtherActor :type "Actor Object Reference") (OtherComp :type "PrimitiveComponent Object Reference") (OtherBodyIndex :type Integer) (bFromSweep :type Boolean) (SweepResult :type "HitResult Structure (by ref)"))
  (bind _asbp_third_person_character (cast `/Game/ThirdPerson/Blueprints/BP_ThirdPersonCharacter` OtherActor))
  (set `/Game/ThirdPerson/Blueprints/BP_ThirdPersonCharacter.InsanerByFlower2D` true _asbp_third_person_character)
  (`/Game/ThirdPerson/Blueprints/BP_ThirdPersonCharacter.InsanityRange` _asbp_third_person_character))

(event `self.Sphere.OnComponentEndOverlap`
  (params (OverlappedComponent :type "PrimitiveComponent Object Reference") (OtherActor :type "Actor Object Reference") (OtherComp :type "PrimitiveComponent Object Reference") (OtherBodyIndex :type Integer))
  (bind _asbp_third_person_character (cast `/Game/ThirdPerson/Blueprints/BP_ThirdPersonCharacter` OtherActor))
  (set `/Game/ThirdPerson/Blueprints/BP_ThirdPersonCharacter.InsanerByFlower2D` true _asbp_third_person_character))

(fn `UserConstructionScript`)