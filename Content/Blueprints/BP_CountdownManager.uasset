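; Countdown manager that runs a scaled game clock down to zero, with start, pause, resume and reset events.
; BeginPlay derives the speed multiplier so 24 countdown hours pass in DayLengthInMinutes real minutes.
; While running and unpaused, Tick subtracts scaled delta time, clamps it to one day and derives Hours and Minutes.
; CountdownFinished clears the run state at zero, but nothing in this Blueprint calls it.
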(event `self.ReceiveTick`
  (params (DeltaSeconds :type "Float (single-precision)"))
  (if (and (`self.isRunning`) (not (`self.isPaused`)))
    (set `self.TimeInSeconds` (`KismetMathLibrary.FClamp` (- (`self.TimeInSeconds`) (* (`GameplayStatics.GetWorldDeltaSeconds`) (`self.SpeedMultiplier`))) 0.0 86400.0))
    (set `self.Hours` (`KismetMathLibrary.FFloor` (/ (`self.TimeInSeconds`) 3600.0)))
    (set `self.Minutes` (`KismetMathLibrary.FFloor` (/ (mod (`self.TimeInSeconds`) 3600.0) 60.0)))))

(event `self.ReceiveBeginPlay`
  (set `self.SpeedMultiplier` (/ 86400.0 (* (`self.DayLengthInMinutes`) 60.0))))

(event `StartCountdown`
  (set `self.isRunning` true)
  (set `self.isPaused` false))

(event `PauseCountdown`
  (set `self.isPaused` true))

(event `ResumeCountdown`
  (set `self.isPaused` false))

(event `ResetCountdown`
  (set `self.TimeInSeconds` (`self.InitialTimeInSeconds`)))

(event `CountdownFinished`
  (if (<= (`self.TimeInSeconds`) 0.0)
    (set `self.isRunning` false)
    (set `self.isPaused` false)
    (`/Engine/EditorBlueprintResources/StandardMacros.DoOnce` false)))

(fn `UserConstructionScript`)