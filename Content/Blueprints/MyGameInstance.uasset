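; Game instance that runs a scaled countdown clock and switches levels when time runs out.
; Init derives a speed multiplier from day length in minutes, which UpdateCountodwn applies to passed-in delta time to compute hours and minutes.
; At zero it resets and opens a Cuts level chosen by current level name, defaulting to UI.
; A collectibles check returns true on the first collected expected key, despite its "all" name.
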(event `self.ReceiveInit`
  (set `self.Speed Multiplier` (/ 86400.0 (* (`self.DayLengthinMinutes`) 60.0)))
  (`self.UpdateCountodwn` 0.0))

(event `StartCountdown`
  ; Countdown
  (set `self.isRunning` true)
  (set `self.isPaused` false))

(event `PauseCountdown`
  ; Countdown
  (set `self.isPaused` true))

(event `ResumeCountdown`
  ; Countdown
  (set `self.isPaused` false))

(event `ResetCountdown`
  ; Countdown
  (set `self.TimeInSeconds` (`self.Initial Time in Seconds`)))

(event `CountdownFinished`
  ; Countdown
  (set `self.isRunning` false)
  (set `self.isPaused` false)
  (`self.ResetCountdown`)
  (bind _returnvalue (`GameplayStatics.GetCurrentLevelName` true))
  (switch `string` _returnvalue
    (:`Default`
      (`GameplayStatics.OpenLevelBySoftObjectPtr` "/Game/FirstPerson/Maps/UI.UI"))
    (:`updated_blockout`
      (`GameplayStatics.OpenLevelBySoftObjectPtr` "/Game/Movie_Dream2/Cuts1.Cuts1"))
    (:`Pools`
      (`GameplayStatics.OpenLevelBySoftObjectPtr` "/Game/Movie_Dream2/Cuts2.Cuts2"))
    (:`second_level`
      (`GameplayStatics.OpenLevelBySoftObjectPtr` "/Game/Movie_Dream2/Cuts3.Cuts3"))))

(fn `AreAllCollectiblesColelcted`
  (params (ExpectedKeys :type "Array of Name"))
  (returns (True :type Boolean))
  (bind _collecteditems (`self.CollectedItems`))
  (for _array_element ExpectedKeys
    (if (and (`BlueprintMapLibrary.Map_Contains` _collecteditems _array_element) (`.ReturnValue` (`BlueprintMapLibrary.Map_Find` _collecteditems _array_element)))
      (return true))))

(fn `UpdateCountodwn`
  (params (DeltaSeconds :type "Float (double-precision)"))
  (locals (NewLocalVar :type "Float (double-precision)" :default 0.0))
  (if (and (`self.isRunning`) (not (`self.isPaused`)))
    (bind _output_get (set `self.TimeInSeconds` (`KismetMathLibrary.FClamp` (- (`self.TimeInSeconds`) (* DeltaSeconds (`self.Speed Multiplier`))) 0.0 (`self.TimeInSeconds`))))
    (set `self.Hours` (`KismetMathLibrary.FFloor` (/ (`self.TimeInSeconds`) 3600.0)))
    (set `self.Minutes` (`KismetMathLibrary.FFloor` (/ (mod (`self.TimeInSeconds`) 3600.0) 60.0)))
    (if (<= _output_get 0.0)
      (`self.CountdownFinished`))))