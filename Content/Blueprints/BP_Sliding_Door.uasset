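; Sliding double door actor that opens when something enters its trigger box and closes when it leaves.
; Box overlap begin plays the OpenCloseDoor timeline and overlap end reverses it, each attaching a stone scrape sound to the box.
; The timeline's DoorTrack drives lerps that slide the left and right door meshes apart along their relative X axis.
; Overlaps are not filtered by actor.
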(event `self.Box.OnComponentBeginOverlap`
  (params (OverlappedComponent :type "PrimitiveComponent Object Reference") (OtherActor :type "Actor Object Reference") (OtherComp :type "PrimitiveComponent Object Reference") (OtherBodyIndex :type Integer) (bFromSweep :type Boolean) (SweepResult :type "HitResult Structure (by ref)"))
  (`GameplayStatics.SpawnSoundAttached` "/Game/Sounds/effects/tomb-door-open-stone-scrape-102748_Cue.tomb-door-open-stone-scrape-102748_Cue" (`self.Box`) "None" (0.0 0.0 0.0) (struct) "KeepRelativeOffset" false 1.0 1.0 0.0 null null)
  (bind (_direction _door_track) (`Timeline|Open/Close door` :!label _label)
    (:`Update`
      (`SceneComponent.K2_SetRelativeLocation` (`self.door left`) (`KismetMathLibrary.MakeVector` (`KismetMathLibrary.Lerp` -150.0 -300.0 _door_track) 0.0 130.0) false false)
      (`SceneComponent.K2_SetRelativeLocation` (`self.door right`) (`KismetMathLibrary.MakeVector` (`KismetMathLibrary.Lerp` 150.0 300.0 _door_track) 0.0 130.0) false false))))

(event `self.Box.OnComponentEndOverlap`
  (params (OverlappedComponent :type "PrimitiveComponent Object Reference") (OtherActor :type "Actor Object Reference") (OtherComp :type "PrimitiveComponent Object Reference") (OtherBodyIndex :type Integer))
  (`GameplayStatics.SpawnSoundAttached` "/Game/Sounds/effects/tomb-door-open-stone-scrape-102748_Cue.tomb-door-open-stone-scrape-102748_Cue" (`self.Box`) "None" (0.0 0.0 0.0) (struct) "KeepRelativeOffset" false 1.0 1.0 0.0 null null)
  (goto _label :!via `Reverse`))

(fn `UserConstructionScript`)