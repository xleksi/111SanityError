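; BP_PlayerScaler is a trigger volume that smoothly resizes the player character to a uniform target scale when they enter it.
; On overlap it stores the BP_ThirdPersonCharacter and its current scale, then restarts a timeline that lerps to TargetScale.
; Each update applies the new scale and calls UpdateScaleState on the character so it can react.
; Leaving the box does nothing, so the new size is not reverted.
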(event `self.ScaleTriggerBox.OnComponentBeginOverlap`
  (params (OverlappedComponent :type "PrimitiveComponent Object Reference") (OtherActor :type "Actor Object Reference") (OtherComp :type "PrimitiveComponent Object Reference") (OtherBodyIndex :type Integer) (bFromSweep :type Boolean) (SweepResult :type "HitResult Structure (by ref)"))
  (bind _targetscale (`self.TargetScale`))
  (bind _playerref (`self.PlayerRef`))
  (bind _asbp_third_person_character (cast `/Game/ThirdPerson/Blueprints/BP_ThirdPersonCharacter` OtherActor))
  (bind _output_get (set `self.PlayerRef` _asbp_third_person_character))
  (bind _output_get_2 (set `self.StartScale` (`self.GetActorScale3D` _output_get)))
  (bind (_direction _newtrack_0) (`Timeline|ScaleTimeline` :`NewTime` (`self.ScalingDuration`) :!via `PlayFromStart`)
    (:`Update`
      (bind _returnvalue (`KismetMathLibrary.VLerp` _output_get_2 (`KismetMathLibrary.MakeVector` _targetscale _targetscale _targetscale) _newtrack_0))
      (`/Engine/EditorBlueprintResources/StandardMacros.IsValid` _playerref
        (:`Is Valid`
          (`self.SetActorScale3D` _playerref _returnvalue)
          (`/Game/ThirdPerson/Blueprints/BP_ThirdPersonCharacter.UpdateScaleState` _playerref))))))

(event `self.ScaleTriggerBox.OnComponentEndOverlap`
  (params (OverlappedComponent :type "PrimitiveComponent Object Reference") (OtherActor :type "Actor Object Reference") (OtherComp :type "PrimitiveComponent Object Reference") (OtherBodyIndex :type Integer)))

(fn `UserConstructionScript`)