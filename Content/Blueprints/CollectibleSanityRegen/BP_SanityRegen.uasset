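; BP_SanityRegen is a collectible pickup that restores the player character's sanity.
; On box overlap with BP_ThirdPersonCharacter, it adds a fixed amount of Sanity clamped to SanityMax and syncs PreviousSanity to the new value.
; It then shows a green blink widget animation and destroys itself.
; The pickup stays in the world if Sanity is already at maximum.
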(event `self.Box.OnComponentBeginOverlap`
  (params (OverlappedComponent :type "PrimitiveComponent Object Reference") (OtherActor :type "Actor Object Reference") (OtherComp :type "PrimitiveComponent Object Reference") (OtherBodyIndex :type Integer) (bFromSweep :type Boolean) (SweepResult :type "HitResult Structure (by ref)"))
  (bind _asbp_third_person_character (cast `/Game/ThirdPerson/Blueprints/BP_ThirdPersonCharacter` OtherActor))
  (if (< (`/Game/ThirdPerson/Blueprints/BP_ThirdPersonCharacter.Sanity` _asbp_third_person_character) (`/Game/ThirdPerson/Blueprints/BP_ThirdPersonCharacter.SanityMax` _asbp_third_person_character))
    (bind _output_get (set `/Game/ThirdPerson/Blueprints/BP_ThirdPersonCharacter.Sanity` (`KismetMathLibrary.FClamp` (+ (`/Game/ThirdPerson/Blueprints/BP_ThirdPersonCharacter.Sanity` _asbp_third_person_character) 25.0) 0.0 (`/Game/ThirdPerson/Blueprints/BP_ThirdPersonCharacter.SanityMax` _asbp_third_person_character)) _asbp_third_person_character))
    (set `/Game/ThirdPerson/Blueprints/BP_ThirdPersonCharacter.PreviousSanity` _output_get _asbp_third_person_character)
    (bind _returnvalue (`|CreateWidget` "/Game/Blueprints/CollectibleSanityRegen/WBP_GreenBlinkEffect.WBP_GreenBlinkEffect_C"))
    (`UserWidget.AddToViewport` _returnvalue 0)
    (`UserWidget.PlayAnimation` _returnvalue (`/Game/Blueprints/CollectibleSanityRegen/WBP_GreenBlinkEffect.BlinkAnim` _returnvalue) 0.0 1 "Forward" 1.0 false)
    (`self.K2_DestroyActor`)))

(fn `UserConstructionScript`)