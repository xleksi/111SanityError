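; BP_Flower2DEnemy4 is a flower enemy that chases the player and harms their sanity on contact.
; Each Tick it caches the player's location, rotates to face them and issues an AI MoveTo to that position.
; Overlapping its sphere collision sets the character's InsanerByFlower2D flag and applies flower damage, triggering Death if Sanity is depleted.
; Ending the overlap clears the flag.
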(event `Rotate`
  (bind _returnvalue (`GameplayStatics.GetPlayerCharacter` 0))
  ; rotate
  (if (`KismetSystemLibrary.IsValid` _returnvalue)
    (`self.K2_SetActorRotation` (`KismetMathLibrary.FindLookAtRotation` (`self.K2_GetActorLocation`) (`self.K2_GetActorLocation` _returnvalue)))))

(event `self.ReceiveTick`
  (params (DeltaSeconds :type "Float (single-precision)"))
  (`self.GetPlayerPosition`)
  (`self.Rotate`)
  (`self.MoveToPlayer`))

(event `self.ReceiveBeginPlay`
  (bind _asbp_third_person_character (cast `/Game/ThirdPerson/Blueprints/BP_ThirdPersonCharacter` (`GameplayStatics.GetPlayerCharacter` 0)))
  (set `self.PlayerRef` _asbp_third_person_character))

(event `self.SphereCollision.OnComponentBeginOverlap`
  (params (OverlappedComponent :type "PrimitiveComponent Object Reference") (OtherActor :type "Actor Object Reference") (OtherComp :type "PrimitiveComponent Object Reference") (OtherBodyIndex :type Integer) (bFromSweep :type Boolean) (SweepResult :type "HitResult Structure (by ref)"))
  (bind _asbp_third_person_character (cast `/Game/ThirdPerson/Blueprints/BP_ThirdPersonCharacter` OtherActor))
  (set `/Game/ThirdPerson/Blueprints/BP_ThirdPersonCharacter.InsanerByFlower2D` true _asbp_third_person_character)
  (`/Game/ThirdPerson/Blueprints/BP_ThirdPersonCharacter.DamageByFlower2d` _asbp_third_person_character)
  (bind _asbp_third_person_character_2 (cast `/Game/ThirdPerson/Blueprints/BP_ThirdPersonCharacter` (`GameplayStatics.GetPlayerPawn` 0)))
  (`/Engine/EditorBlueprintResources/StandardMacros.IsValid` _asbp_third_person_character_2
    (:`Is Valid`
      (if (<= (`/Game/ThirdPerson/Blueprints/BP_ThirdPersonCharacter.Sanity` _asbp_third_person_character_2) 0.0)
        (`/Game/ThirdPerson/Blueprints/BP_ThirdPersonCharacter.Death` _asbp_third_person_character_2)))))

(event `self.SphereCollision.OnComponentEndOverlap`
  (params (OverlappedComponent :type "PrimitiveComponent Object Reference") (OtherActor :type "Actor Object Reference") (OtherComp :type "PrimitiveComponent Object Reference") (OtherBodyIndex :type Integer))
  (bind _asbp_third_person_character (cast `/Game/ThirdPerson/Blueprints/BP_ThirdPersonCharacter` OtherActor))
  (set `/Game/ThirdPerson/Blueprints/BP_ThirdPersonCharacter.InsanerByFlower2D` false _asbp_third_person_character))

(event `MoveToPlayer`
  (bind _asbp_third_person_character (cast `/Game/ThirdPerson/Blueprints/BP_ThirdPersonCharacter` (`GameplayStatics.GetPlayerCharacter` 0)))
  (`/Engine/EditorBlueprintResources/StandardMacros.IsValid` _asbp_third_person_character
    (:`Is Valid`
      (`|AIMoveTo` self (`self.PlayerPos`) null))))

(event `GetPlayerPosition`
  (bind _playerref (`self.PlayerRef`)
    (:`then`
      (set `self.PlayerPos` (`self.K2_GetActorLocation` _playerref)))
    (:`else`)))

(fn `UserConstructionScript`)