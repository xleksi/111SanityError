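; BP_allow_enemyMovment is a trigger that holds the Flowerman enemy in place until the player enters its area.
; On BeginPlay it disables movement on the referenced Flowerman's CharacterMovement component.
; When a BP_ThirdPersonCharacter overlaps the BoxCollitions box, it sets that movement mode back to Walking, with validity checks guarding both steps.
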(event `self.ReceiveBeginPlay`
  (if (`KismetSystemLibrary.IsValid` (`self.Flowerman`))
    (`CharacterMovementComponent.DisableMovement` (`Character.CharacterMovement` (`self.Flowerman`)))))

(event `self.Box collitions.OnComponentBeginOverlap`
  (params (OverlappedComponent :type "PrimitiveComponent Object Reference") (OtherActor :type "Actor Object Reference") (OtherComp :type "PrimitiveComponent Object Reference") (OtherBodyIndex :type Integer) (bFromSweep :type Boolean) (SweepResult :type "HitResult Structure (by ref)"))
  (cast `/Game/ThirdPerson/Blueprints/BP_ThirdPersonCharacter` OtherActor)
  (bind _flowerman (`self.Flowerman`)
    (:`then`
      (`CharacterMovementComponent.SetMovementMode` (`Character.CharacterMovement` _flowerman) "MOVE_Walking" 0))
    (:`else`)))

(fn `UserConstructionScript`)