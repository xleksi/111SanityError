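; BP_Key is a collectible key that the player picks up through an Interact event.
; A Box trigger shows a Widget component while the player's third-person character overlaps it and hides it when the character leaves.
; On Interact, it calls CollectKeyMessage on a referenced Door, destroys itself and prints a green confirmation message.
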(event `self.ReceiveBeginPlay`
  (bind _asbp_third_person_character (cast `/Game/ThirdPerson/Blueprints/BP_ThirdPersonCharacter` (`GameplayStatics.GetPlayerCharacter` 0)))
  (set `self.As BP Third Person Character` _asbp_third_person_character))

(event `self.Box.OnComponentBeginOverlap`
  (params (OverlappedComponent :type "PrimitiveComponent Object Reference") (OtherActor :type "Actor Object Reference") (OtherComp :type "PrimitiveComponent Object Reference") (OtherBodyIndex :type Integer) (bFromSweep :type Boolean) (SweepResult :type "HitResult Structure (by ref)"))
  (if (== OtherActor (`self.As BP Third Person Character`))
    (`SceneComponent.SetVisibility` (`self.Widget`) true false)))

(event `self.Box.OnComponentEndOverlap`
  (params (OverlappedComponent :type "PrimitiveComponent Object Reference") (OtherActor :type "Actor Object Reference") (OtherComp :type "PrimitiveComponent Object Reference") (OtherBodyIndex :type Integer))
  (if (== OtherActor (`self.As BP Third Person Character`))
    (`SceneComponent.SetVisibility` (`self.Widget`) false false)))

(event `/Game/Blueprints/Interfaces/BPI_Interact.Interact`
  (message `/Game/Blueprints/Interfaces/BPI_Door.Collect Key` (`self.Door`))
  (`self.K2_DestroyActor`)
  (`KismetSystemLibrary.PrintString` "You received a KEY" true true (struct :`G` 1.0 :`B` 0.123976 :`A` 1.0)))

(fn `UserConstructionScript`)