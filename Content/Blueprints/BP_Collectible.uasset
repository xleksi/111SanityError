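; BP_Collectible is a pickup that stays collected once the player character takes it.
; Overlapping its sphere records its CollectibleID in the CollectedItems map on MyGameInstance, plays a sound, prints a found message and destroys the actor.
; On BeginPlay it looks up that ID in the map and destroys itself if already collected, so state carries across level loads within a session.
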(event `self.ReceiveBeginPlay`
  (bind _asmy_game_instance (cast `/Game/Blueprints/MyGameInstance` (`GameplayStatics.GetGameInstance`)))
  (set `self.CollectibleID` (`self.CollectibleID`))
  (if (`BlueprintMapLibrary.Map_Contains` (`/Game/Blueprints/MyGameInstance.CollectedItems` _asmy_game_instance) (`self.CollectibleID`))
    (if (`.ReturnValue` (`BlueprintMapLibrary.Map_Find` (`/Game/Blueprints/MyGameInstance.CollectedItems` _asmy_game_instance) (`self.CollectibleID`)))
      (`self.K2_DestroyActor`))))

(event `self.Sphere.OnComponentBeginOverlap`
  (params (OverlappedComponent :type "PrimitiveComponent Object Reference") (OtherActor :type "Actor Object Reference") (OtherComp :type "PrimitiveComponent Object Reference") (OtherBodyIndex :type Integer) (bFromSweep :type Boolean) (SweepResult :type "HitResult Structure (by ref)"))
  (cast `/Game/ThirdPerson/Blueprints/BP_ThirdPersonCharacter` OtherActor)
  (bind _asmy_game_instance (cast `/Game/Blueprints/MyGameInstance` (`GameplayStatics.GetGameInstance`)))
  (`BlueprintMapLibrary.Map_Add` (`/Game/Blueprints/MyGameInstance.CollectedItems` _asmy_game_instance) (`self.CollectibleID`) true)
  (`GameplayStatics.PlaySound2D` "/Engine/EditorSounds/GamePreview/PossessPlayer.PossessPlayer" 1.0 1.0 0.0 null null)
  (`KismetSystemLibrary.PrintString` (`KismetStringLibrary.Concat_StrStr` "Found McGuffin #" (`KismetStringLibrary.Conv_NameToString` (`self.CollectibleID`))) true true (struct :`G` 1.0 :`B` 0.226385 :`A` 1.0))
  (`self.K2_DestroyActor`))

(fn `UserConstructionScript`)