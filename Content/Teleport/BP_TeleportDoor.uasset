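; Teleport door actor that moves a BP_ThirdPersonCharacter when it overlaps the Trigger component.
; The character's PlayerColor indexes TeleportTargets, so each color has its own destination.
; The target location is transformed by the character's current transform, making it a player-relative offset, while the target rotation is applied directly.
; Disconnected leftover nodes hold an older per-color switch that never runs.
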(event `self.Trigger.OnComponentBeginOverlap`
  (params (OverlappedComponent :type "PrimitiveComponent Object Reference") (OtherActor :type "Actor Object Reference") (OtherComp :type "PrimitiveComponent Object Reference") (OtherBodyIndex :type Integer) (bFromSweep :type Boolean) (SweepResult :type "HitResult Structure (by ref)"))
  (bind (_output_location _output_rotation) (`KismetMathLibrary.BreakTransform` (`|GetArrayItem` (`self.TeleportTargets`) (`KismetMathLibrary.Conv_ByteToInt` (`/Game/ThirdPerson/Blueprints/BP_ThirdPersonCharacter.PlayerColor` (`self.PlayerRef`))))))
  (bind _asbp_third_person_character (cast `/Game/ThirdPerson/Blueprints/BP_ThirdPersonCharacter` OtherActor))
  (bind _output_get (set `self.PlayerRef` _asbp_third_person_character))
  (`self.K2_SetActorLocationAndRotation` _output_get (`KismetMathLibrary.TransformLocation` (`self.GetTransform` (`self.PlayerRef`)) _output_location) _output_rotation false true))

(fn `UserConstructionScript`)