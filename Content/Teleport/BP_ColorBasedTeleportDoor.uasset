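; Teleport door actor that moves the third-person character to a destination chosen by the player's current color.
; On trigger overlap, it casts to BP_ThirdPersonCharacter, stores the reference, and indexes TeleportTargets with PlayerColor from MyGameInstance.
; The selected target's location is rotated by its rotation and added to the player's position, making the teleport a relative offset.
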(event `self.Trigger.OnComponentBeginOverlap`
  (params (OverlappedComponent :type "PrimitiveComponent Object Reference") (OtherActor :type "Actor Object Reference") (OtherComp :type "PrimitiveComponent Object Reference") (OtherBodyIndex :type Integer) (bFromSweep :type Boolean) (SweepResult :type "HitResult Structure (by ref)"))
  (bind _returnvalue_location (`KismetMathLibrary.BreakTransform` (`self.GetTransform` (`self.PlayerRef`))))
  (bind (_output_location _output_rotation) (`KismetMathLibrary.BreakTransform` (`|GetArrayItem` (`self.TeleportTargets`) (`KismetMathLibrary.Conv_ByteToInt` (`/Game/Blueprints/MyGameInstance.PlayerColor` (cast `/Game/Blueprints/MyGameInstance` (`GameplayStatics.GetGameInstance`) :!pure true))))))
  (bind _asbp_third_person_character (cast `/Game/ThirdPerson/Blueprints/BP_ThirdPersonCharacter` OtherActor))
  (bind _output_get (set `self.PlayerRef` _asbp_third_person_character))
  (`self.K2_SetActorLocationAndRotation` :`self` _output_get :`NewLocation` (`KismetMathLibrary.TransformLocation` (`KismetMathLibrary.MakeTransform` _returnvalue_location _output_rotation) _output_location) :`bTeleport` true))

(fn `UserConstructionScript`)