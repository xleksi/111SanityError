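; Character component that lets BP_ThirdPersonCharacter grab, carry and throw physics objects from its first-person camera.
; Holding Activate line-traces for a body under the weight limit and attaches it to the PhysicsHandle.
; A self-rescheduling timer keeps the handle target ahead of the camera, even rescheduling after release.
; Releasing zeroes the object's velocity, Confirm throws it forward, and the player-color switch and capsule collision toggles do nothing.
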(event `self.ReceiveBeginPlay`
  (bind _asbp_third_person_character (cast `/Game/ThirdPerson/Blueprints/BP_ThirdPersonCharacter` (`self.GetOwner`)))
  (bind _output_get (set `self.PlayerRef` _asbp_third_person_character))
  (set `self.First Person Camera` (`/Game/ThirdPerson/Blueprints/BP_ThirdPersonCharacter.FirstPersonCamera` _output_get))
  (set `self.Physics Handle` (`/Game/ThirdPerson/Blueprints/BP_ThirdPersonCharacter.PhysicsHandle` _output_get)))

(event `EnhancedInput|/Game/ThirdPerson/Input/Actions/IA_Activate`
  (params (ActionValue :type Boolean) (ElapsedSeconds :type "Float (double-precision)") (TriggeredSeconds :type "Float (double-precision)") (InputAction :type "InputAction Object Reference" :default "/Game/ThirdPerson/Input/Actions/IA_Activate.IA_Activate"))
  (bind _first_person_camera (`self.First Person Camera`))
  (bind _physics_handle (`self.Physics Handle`))
  (bind _returnvalue (`SceneComponent.K2_GetComponentLocation` _first_person_camera))
  ; Geabbing Handler
  (:`Started`
    (if (not (`self.isHolding`))
      (switch `/Game/ThirdPerson/E_PlayerColor` (`/Game/Blueprints/MyGameInstance.PlayerColor` (cast `/Game/Blueprints/MyGameInstance` (`GameplayStatics.GetGameInstance`) :!pure true))
        (:`NewEnumerator0`
          _)
        (:`NewEnumerator1`
          _)
        (:`NewEnumerator2`
          _)
        (:`NewEnumerator3`
          _))
      (bind (_outhit _returnvalue_2) (`KismetSystemLibrary.LineTraceSingleForObjects` :`Start` _returnvalue :`End` (+ _returnvalue (* (`SceneComponent.GetForwardVector` _first_person_camera) (`self.GrabbingDistance`))) :`ObjectTypes` (`|MakeArray` "ObjectTypeQuery4" :!type "EObjectTypeQuery Enum") :`DrawDebugType` "Persistent"))
      (if _returnvalue_2
        (if (<= (`PrimitiveComponent.GetMass` (`.HitComponent` (`GameplayStatics.BreakHitResult` _outhit))) (`self.MaxGrabWeight`))
          (`PhysicsHandleComponent.GrabComponentAtLocationWithRotation` :`self` (`self.Physics Handle`) :`Component` (`.HitComponent` (`GameplayStatics.BreakHitResult` _outhit)) :`Location` (`.Location` (`GameplayStatics.BreakHitResult` _outhit)))
          (`self.UpdateLocation`)
          (set `self.isHolding` true)))))
  (:`Completed`
    (if (`self.isHolding`)
      (`PhysicsHandleComponent.ReleaseComponent` _physics_handle)
      (`PhysicsHandleComponent.SetLinearDamping` _physics_handle 50.0)
      (`PrimitiveComponent.SetPhysicsLinearVelocity` (`.HitComponent` (`GameplayStatics.BreakHitResult` _outhit)) (0.0 0.0 0.0) false "None")
      (`PrimitiveComponent.SetPhysicsAngularVelocityInDegrees` (`.HitComponent` (`GameplayStatics.BreakHitResult` _outhit)) (0.0 0.0 0.0) false "None")
      (set `self.isHolding` false))))

(event `EnhancedInput|/Game/ThirdPerson/Input/Actions/IA_Confirm`
  (params (ActionValue :type Boolean) (ElapsedSeconds :type "Float (double-precision)") (TriggeredSeconds :type "Float (double-precision)") (InputAction :type "InputAction Object Reference" :default "/Game/ThirdPerson/Input/Actions/IA_Confirm.IA_Confirm"))
  (:`Triggered`
    (if (`self.isHolding`)
      (`PhysicsHandleComponent.ReleaseComponent` (`self.Physics Handle`))
      (`/Engine/EditorBlueprintResources/StandardMacros.IsValid` (`.HitComponent` (`GameplayStatics.BreakHitResult` (stale `EnhancedInput|/Game/ThirdPerson/Input/Actions/IA_Activate` _outhit)))
        (:`Is Valid`
          (`PrimitiveComponent.SetPhysicsLinearVelocity` (`.HitComponent` (`GameplayStatics.BreakHitResult` (stale `EnhancedInput|/Game/ThirdPerson/Input/Actions/IA_Activate` _outhit))) (* (`SceneComponent.GetForwardVector` (`self.First Person Camera`)) (`self.ThrowForce`)) false "None")
          (set `self.isHolding` false))))))

(event `UpdateLocation`
  (bind _first_person_camera (`self.First Person Camera`))
  (bind _returnvalue (`SceneComponent.GetForwardVector` _first_person_camera))
  ; Update Location
  (`KismetSystemLibrary.K2_SetTimerDelegate` (delegate `UpdateLocation`) 0.01)
  (if (`self.isHolding`)
    (`PhysicsHandleComponent.SetTargetLocationAndRotation` (`self.Physics Handle`) (+ (`SceneComponent.K2_GetComponentLocation` _first_person_camera) (* _returnvalue (`self.GrabbingDistance`))) (`KismetMathLibrary.Conv_VectorToRotator` _returnvalue))))