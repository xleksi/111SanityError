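; BPC_ColorManager is a component on the third-person character that applies the material and ability tied to the player's current color.
; It caches its owning character on BeginPlay, and ChangePlayerColor switches on PlayerColor to set or reset the material and jump count, with Red granting a double jump.
; It then calls UpdateCollision, which gives Blue a walk-through-walls collision profile on the capsule and every other color the Pawn profile.
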(event `self.ReceiveBeginPlay`
  (set `self.PlayerRef` (cast `/Game/ThirdPerson/Blueprints/BP_ThirdPersonCharacter` (`self.GetOwner`) :!pure true)))

(fn `ChangePlayerColor`
  (bind _playerref (`self.PlayerRef`))
  (bind _playerref_2 (`self.PlayerRef`))
  (bind _playerref_3 (`self.PlayerRef`))
  (switch `/Game/ThirdPerson/E_PlayerColor` (`/Game/ThirdPerson/Blueprints/BP_ThirdPersonCharacter.PlayerColor` (`self.PlayerRef`))
    (:`NewEnumerator0`
      (`/Game/ThirdPerson/Blueprints/BP_ThirdPersonCharacter.ResetCharacterMaterial` _playerref)
      (set `Character.JumpMaxCount` 1 _playerref))
    (:`NewEnumerator1`
      (`/Game/ThirdPerson/Blueprints/BP_ThirdPersonCharacter.SetCharacterMaterial` _playerref_2 "/Engine/EditorResources/FieldNodes/_Resources/M_FieldVolumePreview.M_FieldVolumePreview")
      (set `Character.JumpMaxCount` 2 _playerref_2))
    (:`NewEnumerator2`
      (`/Game/ThirdPerson/Blueprints/BP_ThirdPersonCharacter.SetCharacterMaterial` _playerref_3 "/Engine/ArtTools/RenderToTexture/Materials/M_RadiusDebugTranslucent.M_RadiusDebugTransLucent")
      (set `Character.JumpMaxCount` 1 _playerref_3 :!label _label))
    (:`NewEnumerator3`
      (`/Game/ThirdPerson/Blueprints/BP_ThirdPersonCharacter.SetCharacterMaterial` (`self.PlayerRef`) "/Engine/EditorResources/FieldNodes/_Resources/M_FieldRadiusPreview.M_FieldRadiusPreview")
      (goto _label)))
  (`self.UpdateCollision`))

(fn `UpdateCollision`
  (bind _playerref (`self.PlayerRef`))
  (bind _capsulecomponent (`Character.CapsuleComponent` _playerref))
  (switch `/Game/ThirdPerson/E_PlayerColor` (`/Game/ThirdPerson/Blueprints/BP_ThirdPersonCharacter.PlayerColor` _playerref)
    (:`NewEnumerator0`
      (`PrimitiveComponent.SetCollisionProfileName` _capsulecomponent "Pawn" true :!label _label))
    (:`NewEnumerator1`
      (goto _label))
    (:`NewEnumerator2`
      (goto _label))
    (:`NewEnumerator3`
      (`PrimitiveComponent.SetCollisionProfileName` _capsulecomponent "WalkThroughWallsAbility" true))))