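; BP_Goon3 is a dialogue NPC that turns to face the player every tick and talks to them once.
; On first box overlap by the third-person character, it shows DemoDialogueWidget with Goon3dl, disables character input and shows the mouse cursor.
; Leaving the box removes the widget, restores game-only input mode and sets DoneOnce, so later overlaps only print a done-talking message.
; Character input and cursor are not reset here, and a camera blend node is unwired.
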(event `self.Box.OnComponentBeginOverlap`
  (params (OverlappedComponent :type "PrimitiveComponent Object Reference") (OtherActor :type "Actor Object Reference") (OtherComp :type "PrimitiveComponent Object Reference") (OtherBodyIndex :type Integer) (bFromSweep :type Boolean) (SweepResult :type "HitResult Structure (by ref)"))
  (bind _asbp_third_person_character (cast `/Game/ThirdPerson/Blueprints/BP_ThirdPersonCharacter` OtherActor))
  (if (`self.doneOnce`)
    (`KismetSystemLibrary.PrintString` "DONE TALKING HERE" true true (struct :`R` 1.0 :`B` 0.200784 :`A` 1.0))
    (else
      (`/Engine/EditorBlueprintResources/StandardMacros.DoOnce` false
        (:`Completed`
          (`WidgetBlueprintLibrary.SetInputMode_GameAndUIEx` (`GameplayStatics.GetPlayerController` 0) null)
          ; start dialogue
          (bind _returnvalue (`|GenericCreateObject` "/DialoguePlugin/UI/DemoDialogueWidget.DemoDialogueWidget_C" "/Game/Characters/DialogueNPC/Goon3/goon3-dl.goon3-dl" null))
          (bind _output_get (set `self.DialogueRef` _returnvalue))
          (`UserWidget.AddToViewport` _output_get 0)
          (`self.DisableInput` _asbp_third_person_character null)
          ;[1 1 1] cant see if checked context sensitive
          (set `PlayerController.bShowMouseCursor` true (`GameplayStatics.GetPlayerController` 0)))))))

(event `self.Box.OnComponentEndOverlap`
  (params (OverlappedComponent :type "PrimitiveComponent Object Reference") (OtherActor :type "Actor Object Reference") (OtherComp :type "PrimitiveComponent Object Reference") (OtherBodyIndex :type Integer))
  (cast `/Game/ThirdPerson/Blueprints/BP_ThirdPersonCharacter` OtherActor)
  (`WidgetBlueprintLibrary.SetInputMode_GameOnly` (`GameplayStatics.GetPlayerController` 0))
  (`Widget.RemoveFromParent` (`self.DialogueRef`))
  (set `self.doneOnce` true))

(event `self.ReceiveTick`
  (params (DeltaSeconds :type "Float (single-precision)"))
  (bind _returnvalue (`GameplayStatics.GetPlayerCharacter` 0))
  (if (`KismetSystemLibrary.IsValid` _returnvalue)
    (`self.K2_SetActorRotation` (`KismetMathLibrary.FindLookAtRotation` (`self.K2_GetActorLocation`) (`self.K2_GetActorLocation` _returnvalue)))))

(fn `UserConstructionScript`)